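; Arrow tower Blueprint that picks the enemy closest to the allied base within its attack range.
; BeginPlay caches the first BP_jidi as the base, and the search event sphere-traces for BP_huaihuai after a short delay.
; FUCEnemyFromBaseDistance selects the target by distance to the base, using remembered values that are never reset here.
; A found target goes to the empty Attattack event; otherwise the search repeats.
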(event Custom|Search_Enemy
  (bind _returnvalue (Transformation|GetActorLocation))
  ;[1 1 1] 搜寻
  (Utilities|FlowControl|Delay 0.5)
  (bind (_outhits _returnvalue_2) (Collision|MultiSphereTraceForObjects _returnvalue _returnvalue (Variables|attribute|Getattacke_Range) (Utilities|Array|MakeArray "ObjectTypeQuery7") false 0 "None"))
  (if _returnvalue_2
    (Utilities|Array|Clear (Variables|gaming|GetSearchEnemyArray))
    (for _array_element _outhits
      (bind _asbp_huaihuai (Utilities|Casting|CastToBP_huaihuai (.HitActor (Collision|BreakHitResult _array_element))))
      (Utilities|Array|Add (Variables|gaming|GetSearchEnemyArray) _asbp_huaihuai))
    (if (>= (Utilities|Array|Length (Variables|gaming|GetSearchEnemyArray)) 1)
      (bind (_hasenemy _nearenemytoattack) (CallFunction|FUCEnemyfromBaseDistance))
      (if _hasenemy
        (CallFunction|Attattack _nearenemytoattack)
        (else
          (CallFunction|SearchEnemy :!label _label)))
      (else
        (goto _label)))
    (else
      (CallFunction|SearchEnemy))))

(event Custom|Attattack
  (params (EnemyToAct :type BP%20Huaihuai%20Object%20Reference)))

(event EventBeginPlay
  (bind _outactors (Actor|GetAllActorsOfClass "/Game/sengling/mesh/jidi/BP_jidi.BP_jidi_C"))
  (Variables|Default|SetalineBase (Utilities|Array|Get(acopy) _outactors)))

(event Collision|EventActorBeginOverlap
  (params (OtherActor :type Actor%20Object%20Reference)))

(event EventTick
  (params (DeltaSeconds :type Float%20%28single-precision%29)))

(fn ConstructionScript)

(fn FUCEnemyfromBaseDistance
  (for _array_element (Variables|gaming|GetSearchEnemyArray)
    (if (<= (Math|Vector|VectorLength (- (Transformation|GetActorLocation (Variables|Default|GetalineBase)) (Transformation|GetActorLocation _array_element))) (LocalVariables|GetenemyDistanceRemember))
      (LocalVariables|SetenemyDistanceRemember (Math|Vector|VectorLength (- (Transformation|GetActorLocation (Variables|Default|GetalineBase)) (Transformation|GetActorLocation _array_element))))
      (LocalVariables|SetnearEnemyRemember _array_element)))
  (return (Utilities|IsValid (LocalVariables|GetnearEnemyRemember)) (LocalVariables|GetnearEnemyRemember)))