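; Test enemy character that seeks out BP_pao towers, attacks them and takes armor-reduced damage until destroyed.
; A sphere trace gathers nearby towers, a distance check picks the nearest, and AI MoveTo approaches it.
; After arrival is requested, a looping timer runs forward box traces until a tower is hit, then starts attacking.
; Random montage sections apply damage on notify and repeat while the target remains valid, then searching resumes.
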(event Custom|Hit%20Taget
  ;[1 1 1] 击中
  (Game|Damage|ApplyDamage (Variables|Gaming|GetRef_AttackTower) (Variables|attribute|GetBase%20Damage) 0 self))

(event Custom|MoveAndSearchTarget
  (bind _returnvalue (Transformation|GetActorLocation))
  (bind (_outhits _returnvalue_2) (Collision|MultiSphereTraceForObjects _returnvalue _returnvalue 2e+03 (Utilities|Array|MakeArray "ObjectTypeQuery8") false 0 "ForDuration"))
  (if _returnvalue_2
    (for _array_element _outhits
      (bind _asbp_pao (Utilities|Casting|CastToBP_pao (.HitActor (Collision|BreakHitResult _array_element))))
      (Utilities|Array|Add (Variables|Default|Getmubiao) _asbp_pao))
    (if (>= (Utilities|Array|Length (Variables|Default|Getmubiao)) 1)
      (bind (_hasenemy _nearenemytoattack) (CallFunction|FUCEnemyfromBaseDistance))
      (if _hasenemy
        (AI|AIMoveTo self "0, 0, 0" (Variables|Gaming|GetRef_AttackTower) (Variables|Default|GetAcceptance%20Radius) false
          (:then
            (Utilities|FlowControl|Delay 1.0)
            (bind _returnvalue_3 (Utilities|Time|SetTimerbyFunctionName 0 "FUC_AttackSarch" 0.5 true))
            (Variables|Gaming|SetSearchTimer _returnvalue_3)))
        (else
          (CallFunction|MoveandSearchTarget :!label _label)))
      (else
        (goto _label)))))

(event Custom|Attack
  (bind _arrackanimcount (Variables|Default|GetArrackAnimCount))
  (bind _returnvalue (Math|Random|RandomIntegerinRange 1 _arrackanimcount))
  (bind _returnvalue_2 (Utilities|String|ToString(Integer) _returnvalue))
  (bind _returnvalue_3 (Utilities|String|Append "Attack" _returnvalue_2))
  (Components|Movement|StopMovementImmediately (Variables|Character|GetCharacterMovement))
  (Variables|Gaming|SetIsAttack? true :!label _label)
  (Animation|Montage|PlayMontage (Variables|Character|GetMesh) (Variables|attribute|GetRef_AttackMontage) 1.0 0.0 (Utilities|String|StringToName _returnvalue_3)
    (:then
      (Development|PrintString _returnvalue_3))
    (:OnCompleted
      (Variables|Gaming|SetIsAttack? false)
      (Utilities|IsValid (Variables|Gaming|GetRef_AttackTower)
        (:Is%20Valid
          (goto _label))
        (:Is%20Not%20Valid
          (CallFunction|MoveandSearchTarget))))
    (:OnNotifyBegin
      (CallFunction|HitTaget))))

(event Custom|EventAnyDamage
  (params (Damage :type Float%20%28single-precision%29) (DamageType :type Damage%20Type%20Object%20Reference) (InstigatedBy :type Controller%20Object%20Reference) (DamageCauser :type Actor%20Object%20Reference))
  (bind _output_get (Variables|attribute|SetEnemy_Health (- (Variables|attribute|GetEnemy_Health) (Math|Float|Clamp(Float) (- Damage (Variables|attribute|GetEnemy_Armor)) 0.1 999.0))))
  (if (<= _output_get 0.0)
    (Variables|Default|SetIS_Death? (<= _output_get 0.0))
    (Actor|DestroyActor)))

(event Game|Damage|EventAnyDamage
  (params (Damage :type Float%20%28single-precision%29) (DamageType :type Damage%20Type%20Object%20Reference) (InstigatedBy :type Controller%20Object%20Reference) (DamageCauser :type Actor%20Object%20Reference))
  ;[1 1 1] 应用伤害
  (bind _output_get (Variables|attribute|SetEnemy_Health (- (Variables|attribute|GetEnemy_Health) (Math|Float|Clamp(Float) (- Damage (Variables|attribute|GetEnemy_Armor)) 0.1 999.0))))
  (if (<= _output_get 0.0)
    (Variables|Default|SetIS_Death? (<= _output_get 0.0))))

(event EventBeginPlay
  (CallFunction|MoveandSearchTarget))

(fn ConstructionScript)

(fn FUCAttackSarch
  (bind _returnvalue (Transformation|GetActorRotation))
  (bind _returnvalue_2 (Transformation|GetActorLocation))
  (bind (_roll _pitch _yaw) (Math|Rotator|BreakRotator _returnvalue))
  ;[1 1 1] 搜寻
  (bind (_outhit _returnvalue_3) (Class|KismetSystemLibrary|BoxTraceSingleforObjects _returnvalue_2 (+ (* (Math|Vector|GetForwardVector (Math|Rotator|MakeRotator _roll _pitch (+ _yaw (Variables|attribute|GetAttack%20Angle)))) (Variables|attribute|GetAttackRange)) _returnvalue_2) "50.000000,50.000000,50.000000" "0, 0, 0" (Utilities|Array|MakeArray "ObjectTypeQuery8") false 0 "Persistent" true))
  (if _returnvalue_3
    (bind _asbp_pao (Utilities|Casting|CastToBP_pao (.HitActor (Collision|BreakHitResult _outhit))))
    (Utilities|Time|ClearandInvalidateTimerbyHandle (Variables|Gaming|GetSearchTimer))
    (Variables|Gaming|SetRef_AttackTower _asbp_pao)
    (CallFunction|Attack)))

(fn FUCEnemyfromBaseDistance
  (for _array_element (Variables|Default|Getmubiao)
    (if (<= (Math|Vector|VectorLength (- (Transformation|GetActorLocation) (Transformation|GetActorLocation _array_element))) (LocalVariables|GetenemyDistanceRemember))
      (LocalVariables|SetenemyDistanceRemember (Math|Vector|VectorLength (- (Transformation|GetActorLocation) (Transformation|GetActorLocation _array_element))))
      (Variables|Gaming|SetRef_AttackTower _array_element)))
  (return (Utilities|IsValid (Variables|Gaming|GetRef_AttackTower)) 0))