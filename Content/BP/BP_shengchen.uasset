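; BP_shengchen is a spawner actor that creates BP_huaihuai actors at the location of an arrow component.
; The construction script adds the arrow as Jiantou, and Tick runs a random few-second Delay before each spawn.
; Each spawn goes into GenerateQuantity through AddUnique, whose returned index sets GenerateYN to stop spawning after five.
; A call to Shengcheng is left unconnected and never runs.
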(event EventBeginPlay)

(event Collision|EventActorBeginOverlap
  (params (OtherActor :type Actor%20Object%20Reference)))

(event EventTick
  (params (DeltaSeconds :type Float%20%28single-precision%29))
  (if (not (Variables|Default|GetGenerate_Y/N))
    (Utilities|FlowControl|Delay (Math|Random|RandomFloatinRange 1.0 4.0))
    (Game|SpawnActorfromClass "/Game/BP/huaihuai/BP_huaihuai.BP_huaihuai_C" (Math|Conversions|ToTransform(Vector) (Transformation|GetWorldLocation (Variables|Default|Getjiantou))) "Undefined" 0 0)
    (bind _returnvalue (Utilities|Array|AddUnique (Variables|Default|GetGenerate%20quantity) 0))
    (Variables|Default|SetGenerate_Y/N (>= _returnvalue 4))))

(fn ConstructionScript
  (bind _returnvalue (AddComponent|AddArrowComponent false))
  (Variables|Default|Setjiantou _returnvalue))