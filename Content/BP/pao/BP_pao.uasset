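; Cannon tower that builds itself, attacks BP_huaihuai enemies and takes armor-reduced damage.
; A delayed, repeating sphere trace gathers enemies in range, then FUCEnemyFromBaseDistance favors the one closest to the allied base.
; Attacks optionally yaw toward the target, spawn the weapon on a fire-montage notify, and repeat while it stays valid.
; Damage updates the health widget; at zero, a BP_Pao_Death replacement fires a radial impulse.
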(event Custom|Search_Enemy
  (bind _returnvalue (Transformation|GetActorLocation))
  ;[1 1 1] 搜寻
  (Utilities|FlowControl|Delay 0.5)
  (bind (_outhits _returnvalue_2) (Collision|MultiSphereTraceForObjects _returnvalue _returnvalue (Variables|attribute|Getattacke_Range) (Utilities|Array|MakeArray "ObjectTypeQuery7") false 0 "ForDuration"))
  (if _returnvalue_2
    (Utilities|Array|Clear (Variables|gaming|GetSearchEnemyArray))
    (for _array_element _outhits
      (bind _asbp_huaihuai (Utilities|Casting|CastToBP_huaihuai (.HitActor (Collision|BreakHitResult _array_element))))
      (Utilities|Array|Add (Variables|gaming|GetSearchEnemyArray) _asbp_huaihuai))
    (if (>= (Utilities|Array|Length (Variables|gaming|GetSearchEnemyArray)) 1)
      (bind (_hasenemy _nearenemytoattack) (CallFunction|FUCEnemyfromBaseDistance))
      (if _hasenemy
        (CallFunction|Attattack _nearenemytoattack)
        (else
          (CallFunction|SearchEnemy :!label _label)))
      (else
        (goto _label)))
    (else
      (Utilities|FlowControl|Sequence
        (:then_0
          (CallFunction|SearchEnemy))
        (:then_1
          (Animation|Montage|PlayMontage (Variables|Default|GetSK_Pao) (Variables|reference|Getref_Montage) 1.0 0.0 "xianzhi"))))))

(event Custom|Attattack
  (params (EnemyToAttack :type BP%20Huaihuai%20Object%20Reference))
  (if (Variables|attribute|GetIsAttackNoTurnBody)
    _
    (else
      (Transformation|SetActorRotation self (Math|Rotator|MakeRotator 0.0 0.0 (.yaw (Math|Rotator|FindLookatRotation (Transformation|GetActorLocation) (Transformation|GetActorLocation (Variables|Gaming|GetenemyToAttack))))))))
  (Animation|Montage|PlayMontage (Variables|Default|GetSK_Pao) (Variables|reference|Getref_Montage) 1.0 0.0 "fire"
    (:then
      (Variables|Gaming|Setis_Attacking? true))
    (:OnCompleted
      (Utilities|FlowControl|Delay (Variables|attribute|GetattackTime))
      (Utilities|IsValid (Variables|Gaming|GetenemyToAttack)
        (:Is%20Valid
          (CallFunction|Attattack))
        (:Is%20Not%20Valid
          (Variables|Gaming|Setis_Attacking? false)
          (CallFunction|SearchEnemy))))
    (:OnNotifyBegin
      (Game|SpawnActorfromClass (Variables|reference|Getref_weaponClass) (Transformation|GetWorldTransform (Variables|Default|GetArrow)) "Undefined" "SelectDefaultAtRuntime" 0 0))))

(event EventBeginPlay
  (Variables|attribute|SetTower_Health (Variables|attribute|GetTower_Health_Max))
  (Animation|Montage|PlayMontage (Variables|Default|GetSK_Pao) (Variables|reference|Getref_Montage) 1.0 0.0 "jianzao"
    (:then
      (bind _outactors (Actor|GetAllActorsOfClass "/Game/sengling/mesh/jidi/BP_jidi.BP_jidi_C"))
      (Variables|Gaming|SetalineBase (Utilities|Array|Get(acopy) _outactors)))
    (:OnCompleted
      (CallFunction|SearchEnemy))))

(event Collision|EventActorBeginOverlap
  (params (OtherActor :type Actor%20Object%20Reference)))

(event EventTick
  (params (DeltaSeconds :type Float%20%28single-precision%29)))

(event Game|Damage|EventAnyDamage
  (params (Damage :type Float%20%28single-precision%29) (DamageType :type Damage%20Type%20Object%20Reference) (InstigatedBy :type Controller%20Object%20Reference) (DamageCauser :type Actor%20Object%20Reference))
  (bind _output_get (Variables|attribute|SetTower_Health (- (Variables|attribute|GetTower_Health) (Math|Float|Clamp(Float) (- Damage (Variables|attribute|GetTower_Armor)) 0.001 999.0))))
  (if (<= _output_get 0.0)
    (bind _returnvalue (Game|SpawnActorfromClass (Variables|attribute|GetRef_DeathClass) (Transformation|GetActorTransform) "Undefined" "SelectDefaultAtRuntime" 0 0))
    (bind _asbp_pao_death (Utilities|Casting|CastToBP_Pao_Death _returnvalue))
    (Transformation|SetRelativeLocation (Variables|/Game/BP/pao/BP_Pao_Death.BP_Pao_Death_C|GetRadialForce _asbp_pao_death) (- (Transformation|GetActorLocation) (Transformation|GetActorLocation DamageCauser)) false false)
    (Class|RadialForceComponent|FireImpulse (Variables|/Game/BP/pao/BP_Pao_Death.BP_Pao_Death_C|GetRadialForce _asbp_pao_death))
    (Actor|DestroyActor)
    (else
      (bind _astower_ui (Utilities|Casting|CastToTower_UI (UserInterface|GetUserWidgetObject (Variables|Default|GetHUD_Tower))))
      (Development|PrintString (Utilities|String|ToString(Float) (stale _output_get_2)))
      (bind _output_get_2 (Variables|/Game/UI/Tower_UI.Tower_UI_C|SetTowerHealthPerCent _astower_ui (/ (Variables|attribute|GetTower_Health) (Variables|attribute|GetTower_Health_Max)))))))

(fn ConstructionScript)

(fn FUCEnemyfromBaseDistance
  (for _array_element (Variables|gaming|GetSearchEnemyArray)
    (if (<= (Math|Vector|VectorLength (- (Transformation|GetActorLocation (Variables|Gaming|GetalineBase)) (Transformation|GetActorLocation _array_element))) (LocalVariables|GetenemyDistanceRemember))
      (LocalVariables|SetenemyDistanceRemember (Math|Vector|VectorLength (- (Transformation|GetActorLocation (Variables|Gaming|GetalineBase)) (Transformation|GetActorLocation _array_element))))
      (Variables|Gaming|SetenemyToAttack _array_element)))
  (return (Utilities|IsValid (Variables|Gaming|GetenemyToAttack)) 0))